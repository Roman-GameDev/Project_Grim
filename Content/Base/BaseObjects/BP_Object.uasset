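; Base world object with configurable mesh, material overrides, optional physics and attached sound, passing damage to its health component.
; When simulating physics, it creates dynamic materials for its meshes and can run a looping timer for impact checks.
; Impact checks use bounds-sized sphere or box traces instead of hit events, choosing an effect by velocity.
; They also add a mass-based downward impulse when a line trace finds no ground.
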(event `self.ReceiveBeginPlay`
  (bind _sound (`self.Sound`)
    (:`then`
      (`GameplayStatics.SpawnSoundAttached` _sound (`self.StaticMesh`) "None" (0.0 0.0 0.0) (struct) "KeepRelativeOffset" false 1.0 1.0 0.0 null null))
    (:`else`
      _))
  (if (`self.Simulate Physics`)
    (`self.Set Mass`)
    (`PrimitiveComponent.SetSimulatePhysics` (`self.StaticMesh`) (`self.Simulate Physics`))
    (for _array_element (`self.Get List Of Scene Components`)
      (bind _asstatic_mesh_component (cast `StaticMeshComponent` _array_element))
      (for (_array_element_2 _array_index) (`MeshComponent.GetMaterials` _asstatic_mesh_component)
        (bind _returnvalue (`KismetMaterialLibrary.CreateDynamicMaterialInstance` _array_element_2))
        (`KismetArrayLibrary.Array_Add` (`self.Materials`) _returnvalue)
        (`PrimitiveComponent.SetMaterial` _asstatic_mesh_component _array_index _returnvalue)))
    (if (`self.Generate Impacts?`)
      (`KismetSystemLibrary.K2_SetTimerDelegate` (`|CreateDelegate` :!event `Check For Impacts`) 0.05 true))))

(event `Play Tumble Sound`
  (`/Engine/EditorBlueprintResources/StandardMacros.DoOnce` false :!label _label
    (:`Completed`
      (`GameplayStatics.PlaySoundAtLocation` null (`SceneComponent.K2_GetComponentLocation` (`self.StaticMesh`)) (struct) 1.0 1.0 0.0 null null null null)
      (`KismetSystemLibrary.K2_SetTimerDelegate` (`|CreateDelegate` :!event `Reset Sound`) 0.3))))

(event `Reset Sound`
  (goto _label :!via `Reset`))

(event `self.StaticMesh.OnComponentHit`
  (params (HitComponent :type "PrimitiveComponent Object Reference") (OtherActor :type "Actor Object Reference") (OtherComp :type "PrimitiveComponent Object Reference") (NormalImpulse :type "Vector Structure") (Hit :type "HitResult Structure (by ref)")))

(fn `Apply Damage`
  (params (`Damage Info` :type "/Game/Base/BaseDamage/Struct_DamageHitResult Structure"))
  (returns (Success :type Boolean))
  (bind _success (`/Game/Base/BaseDamage/Health/Comp_Health.Apply Damage` (`self.Comp_Health`) `Damage Info`))
  (return _success))

(fn `Check For Impacts`
  (bind _draw_debug_type (`self.Draw Debug Type`))
  (bind (_origin _boxextent) (`KismetSystemLibrary.GetComponentBounds` (`self.StaticMesh`)))
  (bind (_origin_2 _boxextent_2 _sphereradius) (`KismetSystemLibrary.GetComponentBounds` (`self.StaticMesh`)))
  (`self.Check If Falling`)
  (if (> (`self.Get Velocity Rating`) 5)
    (switch `/Game/Base/BaseObjects/Enum_TraceTypes` (`self.Trace Type`)
      (:`NewEnumerator0`
        (bind (_outhit _returnvalue) (`KismetSystemLibrary.SphereTraceSingle` :`Start` _origin_2 :`End` (- _origin_2 (0.0 0.0 1.0)) :`Radius` _sphereradius :`TraceChannel` "TraceTypeQuery1" :`DrawDebugType` _draw_debug_type :`DrawTime` 0.05))
        (if _returnvalue
          (`self.Impact Effect` _outhit (`self.Get Velocity Rating`))))
      (:`NewEnumerator1`
        (bind (_outhit_2 _returnvalue_2) (`KismetSystemLibrary.BoxTraceSingle` :`Start` _origin :`End` (- _origin (0.0 0.0 1.0)) :`HalfSize` _boxextent :`Orientation` (`SceneComponent.K2_GetComponentRotation` (`self.StaticMesh`)) :`TraceChannel` "TraceTypeQuery1" :`DrawDebugType` _draw_debug_type :`DrawTime` 0.05))
        (if _returnvalue_2
          (`self.Impact Effect` _outhit_2 (`self.Get Velocity Rating`)))))))

(fn `Check If Falling`
  (bind _returnvalue (`self.K2_GetActorLocation`))
  (bind _z (.z (`.BoxExtent` (`KismetSystemLibrary.GetComponentBounds` (`self.StaticMesh`)))))
  (bind (_outhit _returnvalue_2) (`KismetSystemLibrary.LineTraceSingle` (+ _returnvalue (`KismetMathLibrary.MakeVector` 0.0 0.0 _z)) (- _returnvalue (`KismetMathLibrary.MakeVector` 0.0 0.0 (+ _z 3.0))) "TraceTypeQuery1"))
  (if (not _returnvalue_2)
    (`PrimitiveComponent.AddImpulse` (`self.StaticMesh`) (`KismetMathLibrary.MakeVector` 0.0 0.0 (* (`self.Mass`) -1.0)) "None" true)))

(fn `Get List Of Scene Components`
  (returns (SC :type "Array of SceneComponent Object Reference"))
  (locals (NewLocalVar :type "Array of SceneComponent Object Reference"))
  (bind _staticmesh (`self.StaticMesh`))
  (bind _output_get (set `local.NewLocalVar` (`SceneComponent.GetChildrenComponents` _staticmesh true)))
  (`KismetArrayLibrary.Array_Add` _output_get _staticmesh)
  (return (`local.NewLocalVar`)))

(fn `Get Mass`
  (returns (Mass :type "Float (double-precision)"))
  (return (`self.Mass`)))

(fn `Get Tags`
  (returns (Tags :type "GameplayTagContainer Structure"))
  (return (`/Game/Base/BaseObjects/Comp_GameplayTagContainer.Container` (`/Game/Base/BaseDamage/Health/Comp_Health.Tag Container` (`self.Comp_Health`)))))

(fn `Get Velocity Rating`
  (returns (Rating :type Integer))
  (bind _returnvalue (`PrimitiveComponent.GetPhysicsLinearVelocity` (`self.StaticMesh`) "None"))
  (return (`KismetMathLibrary.FTrunc` (/ (`KismetMathLibrary.VSize` _returnvalue) 100.0))))

(fn `Impact Effect`
  (params (Hit :type "HitResult Structure") (InputPin :type Integer))
  (`/Game/Base/BFL_General.Play Effect` Hit (select `bool` (> InputPin 15) :`false` "NewEnumerator1" :`true` "NewEnumerator3" :!type "/Game/Base/BasePhysMaterialSystem/Enum_ImpactTypes Enum"))
  (return))

(fn `Set Mass`
  (bind _staticmesh (`self.StaticMesh`))
  (`PrimitiveComponent.SetMassScale` _staticmesh "None" 10000.0)
  (`PrimitiveComponent.SetAllMassScale` _staticmesh 1000.0))

(fn `UserConstructionScript`
  (bind _staticmesh (`self.StaticMesh`))
  (bind _override_materials (`self.Override Materials`))
  (`parent.UserConstructionScript`)
  (`self.Set Mass`)
  (bind _mesh (`self.Mesh`)
    (:`then`
      (`StaticMeshComponent.SetStaticMesh` _staticmesh _mesh))
    (:`else`
      _))
  (`PrimitiveComponent.SetSimulatePhysics` _staticmesh (`self.Simulate Physics`))
  (if (`KismetArrayLibrary.Array_IsNotEmpty` _override_materials)
    (for (_array_element _array_index) _override_materials
      (`PrimitiveComponent.SetMaterial` (`self.StaticMesh`) _array_index _array_element))))