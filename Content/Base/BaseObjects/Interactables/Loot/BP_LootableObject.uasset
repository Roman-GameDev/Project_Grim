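; Base lootable world object that holds item data and can be picked up through interaction.
; The construction script rolls a random item from its loot table when no valid item data is set.
; Interact passes the object and item to the interactor's pickup message and, on success, sets the mesh to ignore a custom trace channel, likely the interaction trace.
; A separate function overwrites the stored item's quantity.
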(fn `Interact`
  (params (Interactor :type "Actor Object Reference") (`Interacting Component` :type "SceneComponent Object Reference"))
  (returns (Success :type Boolean))
  (bind _return (message `/Game/Base/BaseObjects/Interactables/BPI_Interactor.Pick Up Item` Interactor self (`self.Item Data`)))
  (if _return
    (`PrimitiveComponent.SetCollisionResponseToChannel` (`self.StaticMesh`) "ECC_GameTraceChannel3" "ECR_Ignore"))
  (return true))

(fn `Modify Quantity`
  (params (Quantity :type Integer))
  (returns (Return :type Boolean))
  (setmembers `/Game/Base/BaseInventory/Data/ST_Item` :`StructRef` (`self.Item Data`) :`Quantity` Quantity)
  (return false))

(fn `UserConstructionScript`
  (`parent.UserConstructionScript`)
  (`/Engine/EditorBlueprintResources/StandardMacros.IsValid` (`.Data_2_F3A1C4BF456F492026C721B9BCBE8DF0` (break `/Game/Base/BaseInventory/Data/ST_Item` (`self.Item Data`)))
    (:`Is Not Valid`
      (set `self.Item Data` (`KismetArrayLibrary.Array_Random` (`self.Loot Table`))))))