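; BP_UpgradeChest is a one-time interactable chest that presents a reward screen when opened.
; Its Interact override proceeds only while the chest is unopened and the parent interaction succeeds.
; It then adds a WB_RewardScreen widget with three choices to the viewport, sets Opened to block reuse, and reports success.
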(fn `Interact`
  (params (Interactor :type "Actor Object Reference") (`Interacting Component` :type "SceneComponent Object Reference"))
  (returns (Success :type Boolean))
  (if (not (`self.Opened?`))
    (bind _success (`parent.Interact` Interactor `Interacting Component`))
    (if _success
      (bind _returnvalue (`|CreateWidget` "/Game/RomansStuff/Rewards/WB_RewardScreen.WB_RewardScreen_C"))
      (`UserWidget.AddToViewport` _returnvalue 0)
      (set `self.Opened?` true)
      (return true))))

(fn `UserConstructionScript`
  (`parent.UserConstructionScript`))