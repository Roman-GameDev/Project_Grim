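; BP_Light is a light fixture with a configurable color and an optional flicker.
; The construction script colors the spotlight, and BeginPlay creates a dynamic material for the bulb mesh so it matches that color.
; ChangeLightColor updates both bulb and spotlight at runtime.
; Flicker uses self-rescheduling random timers to briefly cut the spotlight and restore a fixed intensity, leaving the bulb material untouched.
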(event `self.ReceiveBeginPlay`
  (`parent.ReceiveBeginPlay`)
  (if (`self.Flicker?`)
    (`KismetSystemLibrary.K2_SetTimerDelegate` (`|CreateDelegate` :!event `Flicker`) 0.1))
  (bind _returnvalue (`KismetMaterialLibrary.CreateDynamicMaterialInstance` null))
  (bind _output_get (set `self.Bulb Material` _returnvalue))
  (`PrimitiveComponent.SetMaterial` (`self.StaticMesh`) 1 _output_get)
  (`MaterialInstanceDynamic.SetVectorParameterValue` (`self.Bulb Material`) "Light Color" (`self.Light Color`)))

(event `Change Light Color`
  (params (Value :type "LinearColor Structure"))
  (bind _output_get (set `self.Light Color` Value))
  (`MaterialInstanceDynamic.SetVectorParameterValue` (`self.Bulb Material`) "Light Color" _output_get)
  (`LightComponent.SetLightColor` (`self.SpotLight`) (`self.Light Color`) true))

(event `Flicker`
  (`LightComponent.SetIntensity` (`self.SpotLight`) 0.0)
  (`KismetSystemLibrary.K2_SetTimerDelegate` (delegate `Reset Flicker`) 0.1)
  (`KismetSystemLibrary.K2_SetTimerDelegate` (delegate `Flicker`) (`KismetMathLibrary.RandomFloatInRange` 0.4 1.0)))

(event `Reset Flicker`
  (`LightComponent.SetIntensity` (`self.SpotLight`) 3000.0))

(fn `UserConstructionScript`
  (`parent.UserConstructionScript`)
  (`LightComponent.SetLightColor` (`self.SpotLight`) (`self.Light Color`) true))