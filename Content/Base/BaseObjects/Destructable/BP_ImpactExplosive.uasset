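; Destructible explosive prop that, once primed, detonates when it touches something.
; Priming marks it damaged and starts a looping timer that sphere-traces the mesh bounds on Visibility, exploding on any hit.
; The explosion spawns an effect, applies player-tagged damage and impulse to radial trace hits, then destroys the actor.
; Taking damage runs the parent logic and sets a short delayed event.
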(event `Prime`
  (set `self.Damaged` true)
  (`KismetSystemLibrary.K2_SetTimerDelegate` (delegate `Check Impact`) 0.05 true))

(event `Check Impact`
  (bind (_origin _boxextent _sphereradius) (`KismetSystemLibrary.GetComponentBounds` (`self.StaticMesh`)))
  (bind (_outhit _returnvalue) (`KismetSystemLibrary.SphereTraceSingle` _origin (- _origin (0.0 0.0 1.0)) _sphereradius "TraceTypeQuery1"))
  (if _returnvalue
    (`self.Explode`)))

(event `Explode`
  (`NiagaraFunctionLibrary.SpawnSystemAtLocation` null (`SceneComponent.K2_GetComponentLocation` (`self.StaticMesh`)))
  (bind _hits_result (`/Game/Base/BFL_General.Explosion Trace` (`SceneComponent.K2_GetComponentLocation` (`self.StaticMesh`)) 300.0 "TraceTypeQuery1" "None" (`|MakeArray` self :!type "Actor Object Reference")))
  (for _array_element _hits_result
    (message `/Game/Base/BaseDamage/Health/BPI_Health.Apply Damage` (`.HitActor` (`GameplayStatics.BreakHitResult` _array_element)) (make `/Game/Base/BaseDamage/Struct_DamageHitResult` (struct) _array_element (struct :`GameplayTags` (struct :`(TagName` "DamageSource.Player") :`(TagName` "DamageTypes.Explosive"))) null 10.0))
    (`/Game/Base/BFL_General.Apply Impulse to Hit` _array_element 1000.0))
  (`self.K2_DestroyActor`))

(fn `Apply Damage`
  (params (`Damage Info` :type "/Game/Base/BaseDamage/Struct_DamageHitResult Structure"))
  (returns (Success :type Boolean))
  (`parent.Apply Damage` `Damage Info`)
  (`KismetSystemLibrary.K2_SetTimerDelegate` (`|CreateDelegate` :!event `Prime`) 0.1)
  (return true))

(fn `UserConstructionScript`
  (`parent.UserConstructionScript`))