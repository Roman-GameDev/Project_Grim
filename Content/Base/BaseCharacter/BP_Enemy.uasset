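; Base enemy character that detects the player, chases and attacks on a cooldown, and carries a random lootable item.
; Proximity starts timed sight checks using tiered facing-and-distance thresholds plus a sphere trace for line of sight.
; Aggro starts looping movement and attack-range timers and alerts nearby actors, which join after their own visibility check.
; Attack, Death and ApplyDamage are empty here; ragdoll death and damage-triggered aggro logic is disconnected.
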(event `self.ReceiveBeginPlay`
  (set `self.Target` (`GameplayStatics.GetPlayerCharacter` 0))
  (set `CharacterMovementComponent.MaxWalkSpeed` (`self.Speed`) (`self.CharacterMovement`)))

(event `/Game/Base/BaseCharacter/BPI_AI.AI Proximity`
  (`self.Target`
    (:`then`
      (`/Engine/EditorBlueprintResources/StandardMacros.DoOnce` false :!label _label
        (:`Completed`
          (`self.Start Checking Sight`))))
    (:`else`)))

(event `Death`)

(event `Start Checking Sight`
  (`KismetSystemLibrary.K2_SetTimerDelegate` (delegate `Check Sight`) 0.2 true)
  (goto _label_2 :!via `Reset`))

(event `Check Sight`
  (if (and (or (`self.Sight Check` -0.5 2500.0) (`self.Sight Check` -0.2 1250.0) (`self.Sight Check` -0.05 700.0) (`self.Sight Check` 1.0 250.0)) (`self.Line of SIght Check`))
    (`KismetSystemLibrary.K2_ClearTimer` null "Check Sight")
    (`/Engine/EditorBlueprintResources/StandardMacros.DoOnce` false :!label _label_2
      (:`Completed`
        (`self.Aggro Towards Player`)))
    (elif (not (< (`self.Get Distance to Target`) 2600.0))
      (`KismetSystemLibrary.K2_ClearTimer` null "Check Sight")
      (goto _label :!via `Reset`))))

(event `Aggro Towards Player`
  (bind _returnvalue (`self.K2_GetActorLocation`))
  (`self.Move Towards Target`)
  (`KismetSystemLibrary.K2_SetTimerDelegate` (delegate `Check Attack Distance`) 0.3 true)
  (`self.On Aggroed`)
  (set `self.IsAggroed?` true)
  (bind (_outhits _returnvalue_2) (`KismetSystemLibrary.SphereTraceMulti` _returnvalue (- _returnvalue (0.0 0.0 1.0)) 600.0 "TraceTypeQuery4"))
  (if _returnvalue_2
    (for _array_element _outhits
      (message `/Game/Base/BaseCharacter/BPI_AI.AI Aggro Towards Player Override` (`.HitActor` (`GameplayStatics.BreakHitResult` _array_element))))))

(event `Check Attack Distance`
  (if (< (`self.Get Distance to Target`) (`self.Attack Distance`))
    (`/Engine/EditorBlueprintResources/StandardMacros.DoOnce` false :!label _label_3
      (:`Completed`
        (`self.Attack`)
        (`KismetSystemLibrary.K2_SetTimerDelegate` (delegate `Attack Delay Timer`) (`self.Attack Delay`))))))

(event `Attack Delay Timer`
  (goto _label_3 :!via `Reset`))

(event `Move Towards Target`
  (if (`self.CanMove?`)
    (`|AIMoveTo` self (0.0 0.0 0.0) (`self.Target`) 50.0 true
      (:`OnSuccess`
        _)
      (:`OnFail`
        _))
    (if (`self.CanMove?`)
      (`KismetSystemLibrary.K2_SetTimerDelegate` (delegate `Move Towards Target`) 0.1))))

(event `Attack`)

(event `/Game/Base/BasePlayer/BPI_Character.Launch Character`
  (params (`Launch Velocity` :type "Vector Structure") (`Override XY` :type Boolean) (`Override Z` :type Boolean))
  (bind _returnvalue (+ (* `Launch Velocity` 3.0) (0.0 0.0 200.0)))
  (`self.Stop Movement`)
  (if (> (`/Game/Base/BaseDamage/Comp_Resource.Current Resource` (`self.Comp_Health`)) 0.0)
    (`self.LaunchCharacter` _returnvalue `Override XY` `Override Z`)
    (else
      (`PrimitiveComponent.AddImpulse` (`self.SkeletalMeshComponentBudgeted`) _returnvalue "None" true))))

(event `/Game/Base/BaseCharacter/BPI_AI.AI Aggro Towards Player Override`
  (bind _returnvalue (`SceneComponent.K2_GetComponentLocation` (`self.Sight`)))
  (if (not (`self.IsAggroed?`))
    (bind _outhit (`KismetSystemLibrary.LineTraceSingle` _returnvalue (`/Game/Base/BFL_General.Convert Trace` _returnvalue (`self.Get Direction to Target` 50.0)) "TraceTypeQuery1"))
    (if (== (`.HitActor` (`GameplayStatics.BreakHitResult` _outhit)) (`self.Target`))
      (`self.Aggro Towards Player`))))

(fn `Apply Damage`
  (params (`Damage Info` :type "/Game/Base/BaseDamage/Struct_DamageHitResult Structure"))
  (returns (Success :type Boolean)))

(fn `Clear Interaction`
  (returns (Success :type Boolean))
  (return false))

(fn `Enable Movement`
  (params (`CanMove?` :type Boolean))
  (bind _output_get (set `self.CanMove?` `CanMove?`))
  (if _output_get
    (`self.Move Towards Target`)
    (set `CharacterMovementComponent.MaxWalkSpeed` (`self.Speed`) (`self.CharacterMovement`))
    (else
      (`Controller.StopMovement` (`self.GetController`))
      (`MovementComponent.StopMovementImmediately` (`self.CharacterMovement`))
      (set `CharacterMovementComponent.MaxWalkSpeed` 0.0 (`self.CharacterMovement`)))))

(fn `Get Direction to Target`
  (params (`Z Mod` :type "Float (double-precision)"))
  (returns (ReturnValue :type "Vector Structure"))
  (return (`KismetMathLibrary.GetDirectionUnitVector` (`SceneComponent.K2_GetComponentLocation` (`self.Sight`)) (+ (`self.K2_GetActorLocation` (`self.Target`)) (`KismetMathLibrary.MakeVector` 0.0 0.0 `Z Mod`)))))

(fn `Get Distance to Target`
  (returns (ReturnValue :type "Float (double-precision)"))
  (return (`KismetMathLibrary.Vector_Distance` (`self.K2_GetActorLocation` (`self.Target`)) (`self.K2_GetActorLocation`))))

(fn `Get Mass`
  (returns (Mass :type "Float (double-precision)"))
  (return 10.0))

(fn `Get Tags`
  (returns (Tags :type "GameplayTagContainer Structure"))
  (return))

(fn `Interact`
  (params (Interactor :type "Actor Object Reference") (`Interacting Component` :type "SceneComponent Object Reference"))
  (returns (Success :type Boolean))
  (bind _return (message `/Game/Base/BaseObjects/Interactables/BPI_Interactor.Pick Up Item` Interactor self (`self.Lootable Item`)))
  (if _return
    (`PrimitiveComponent.SetCollisionResponseToChannel` (`self.SkeletalMeshComponentBudgeted`) "ECC_GameTraceChannel3" "ECR_Ignore"))
  (return true))

(fn `Line of SIght Check`
  (returns (ReturnValue :type Boolean))
  (bind _returnvalue (`SceneComponent.K2_GetComponentLocation` (`self.Sight`)))
  (bind (_outhit _returnvalue_2) (`KismetSystemLibrary.SphereTraceSingle` _returnvalue (`/Game/Base/BFL_General.Convert Trace` _returnvalue (`self.Get Direction to Target` 50.0) 1250.0) 10.0 "TraceTypeQuery1"))
  (if _returnvalue_2
    (return (== (`.HitActor` (`GameplayStatics.BreakHitResult` _outhit)) (`self.Target`)))
    (else
      (return false))))

(fn `Modify Quantity`
  (params (Quantity :type Integer))
  (returns (Return :type Boolean))
  (setmembers `/Game/Base/BaseInventory/Data/ST_Item` :`StructRef` (`self.Lootable Item`) :`Quantity` Quantity)
  (return false))

(fn `Play Voiceline`
  (params (Voiceline :type "SoundWave Object Reference") (`Override?` :type Boolean))
  (bind _voice_comp (`self.Voice Comp`))
  (if `Override?`
    (`self.Stop Voiceline`))
  (bind _voice_comp_2 (`self.Voice Comp`)
    (:`then`
      (if (or (not (`AudioComponent.IsPlaying` _voice_comp_2)) (`local.Override?`))
        (if (or (> (`/Game/Base/BaseDamage/Comp_Resource.Current Resource` (`self.Comp_Health`)) 0.0) (`local.Override?`)) :!label _label
          (`self.Voice Comp`
            (:`then`
              _)
            (:`else`
              (bind _returnvalue (`GameplayStatics.SpawnSoundAttached` (`self.Voice`) (`self.Sight`) "None" (0.0 0.0 0.0) (struct) "KeepRelativeOffset" false 1.0 1.0 0.0 null null))
              (set `self.Voice Comp` _returnvalue)))
          (`AudioComponent.SetFloatParameter` _voice_comp "Pitch" (`self.Voice Pitch`))
          (`AudioComponent.SetWaveParameter` _voice_comp "sound" (`local.Voiceline`))
          (`AudioComponent.Play` _voice_comp 0.0))))
    (:`else`
      (goto _label))))

(fn `Sight Check`
  (params (Angle :type "Float (double-precision)") (Distance :type "Float (double-precision)"))
  (returns (ReturnValue :type Boolean))
  (return (and (< (`KismetMathLibrary.Dot_VectorVector` (`self.GetActorForwardVector`) (`self.GetActorForwardVector` (`self.Target`))) Angle) (< (`self.Get Distance to Target`) Distance))))

(fn `Stop Movement`
  (bind _charactermovement (`self.CharacterMovement`))
  (`MovementComponent.StopMovementImmediately` _charactermovement)
  (set `MovementComponent.Velocity` (0.0 0.0 0.0) _charactermovement))

(fn `Stop Voiceline`
  (bind _voice_comp (`self.Voice Comp`)
    (:`then`
      (`AudioComponent.Stop` _voice_comp))
    (:`else`
      _))
  (return))

(fn `UserConstructionScript`
  (set `self.Voice Pitch` (`KismetMathLibrary.RandomFloatInRange` -3.0 3.0))
  (`/Engine/EditorBlueprintResources/StandardMacros.IsValid` (`.Data_2_F3A1C4BF456F492026C721B9BCBE8DF0` (break `/Game/Base/BaseInventory/Data/ST_Item` (`self.Lootable Item`)))
    (:`Is Not Valid`
      (set `self.Lootable Item` (`KismetArrayLibrary.Array_Random` (`self.Loot Table`))))))