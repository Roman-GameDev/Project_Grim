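; BP_Explosion is a one-shot explosion actor that damages and pushes what it hits within a radius, then destroys itself.
; On BeginPlay it plays a world camera shake and runs an explosion trace.
; Each hit receives a damage message crediting the Spawner, a hit effect and an impulse, with damage and force scaled down linearly by distance.
; It also spawns a VFX system that receives the radius as a parameter.
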(event `self.ReceiveBeginPlay`
  (bind _radius (`self.Radius`))
  (`GameplayStatics.PlayWorldCameraShake` "/Game/Project/LCS_Explosion.LCS_Explosion_C" (`self.K2_GetActorLocation`) 0.0 (* (`self.Radius`) 2.0) 0.5 true)
  (bind _hits_result (`/Game/Base/BFL_General.Explosion Trace` (`self.K2_GetActorLocation`) _radius))
  (for _array_element _hits_result
    (bind (_bblockinghit _binitialoverlap _time _distance _location _impactpoint _normal _impactnormal _physmat _hitactor) (`GameplayStatics.BreakHitResult` _array_element))
    (bind _returnvalue (`KismetMathLibrary.MapRangeClamped` (/ _distance _radius) 0.0 1.0 (`self.Damage`)))
    (message `/Game/Base/BaseDamage/Health/BPI_Health.Apply Damage` _hitactor (make `/Game/Base/BaseDamage/Struct_DamageHitResult` (make `/Game/Base/BaseDamage/Struct_Damage` _returnvalue 1.0) _array_element (`self.Damage Info Hit Tags`) (`self.Spawner`)))
    (`/Game/Base/BFL_General.Play Effect` _array_element "NewEnumerator3")
    (`/Game/Base/BFL_General.Apply Impulse to Hit` _array_element (* _returnvalue 10.0)))
  (`|ExecutionSequence`
    (:`then_0`
      (bind _returnvalue_2 (`NiagaraFunctionLibrary.SpawnSystemAtLocation` (`self.VFX`) (`self.K2_GetActorLocation`)))
      (`NiagaraComponent.SetVariableFloat` _returnvalue_2 "Radius" (`self.Radius`)))
    (:`then_1`
      (`self.K2_DestroyActor`))))

(fn `UserConstructionScript`)