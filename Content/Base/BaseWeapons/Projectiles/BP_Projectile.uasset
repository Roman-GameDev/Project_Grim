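; Base weapon projectile configured by a Data struct for mesh, trail, launch speed, spin, ricochets and explosions.
; A physics sphere flies with timer-driven gravity impulses, while looping sphere traces from mesh sockets detect head and optional body hits.
; An initial forward trace catches close-range hits at spawn.
; Hits apply fixed damage and impulse, then either ricochet along the surface normal or stop, explode and either stick or drop as physics debris.
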(event `self.ReceiveBeginPlay`
  (bind _data (`self.Data`))
  (bind _speed (`/Game/Base/BaseWeapons/Projectiles/DA_Projectile.Speed` (`self.Data`)))
  (`|ExecutionSequence`
    (:`then_0`
      (`KismetSystemLibrary.K2_SetTimerDelegate` (`|CreateDelegate` :!event `Start Trace`) 0.01 false true)
      (`self.Start Rotation`)
      (`self.Set Projectile Velocity` (`KismetMathLibrary.Conv_RotatorToVector` (`self.K2_GetActorRotation`)) (`KismetMathLibrary.Lerp` (/ _speed 2.0) _speed (`self.Spawn Force Ratio`)))
      (bind _returnvalue (`KismetSystemLibrary.K2_SetTimerDelegate` (`|CreateDelegate` :!event `Fake Physics`) 0.05 true))
      (set `self.Physics` _returnvalue)
      (if (not (`/Game/Base/BaseWeapons/Projectiles/DA_Projectile.Can Be Picked Up?` _data))
        (`KismetSystemLibrary.K2_SetTimerDelegate` (`|CreateDelegate` :!event `Destroy Projectile`) (`/Game/Base/BaseWeapons/Projectiles/DA_Projectile.Lifetime` _data))))
    (:`then_1`
      (`self.Initial Trace`)
      (`KismetSystemLibrary.K2_SetTimer` null "Clear Ignores" 0.2))))

(event `Destroy Actor`
  (params (PSystem :type "NiagaraComponent Object Reference"))
  (`self.K2_DestroyActor`))

(event `Trace for Hit`
  (if (`self.IsActive?`)
    (`self.K2_SetActorRotation` (`KismetMathLibrary.Conv_VectorToRotator` (`self.Get Direction`)))
    (bind _success (`self.Trace Head`))
    (if (and (not _success) (`/Game/Base/BaseWeapons/Projectiles/DA_Projectile.Trace Body?` (`self.Data`)))
      (`self.Trace Body`))))

(event `Fake Physics`
  (`PrimitiveComponent.AddImpulse` (`self.Sphere`) (`KismetMathLibrary.MakeVector` 0.0 0.0 (* (`/Game/Base/BaseWeapons/Projectiles/DA_Projectile.Gravity` (`self.Data`)) -200.0)) "None" true))

(fn `Clear Ignores`
  (`KismetArrayLibrary.Array_Clear` (`self.Actors to Ignore`)))

(fn `Destroy Projectile`
  (locals (`Bound?` :type Boolean))
  (bind _niagara (`self.Niagara`)
    (:`then`
      (if (`ActorComponent.IsActive` _niagara)
        (`ActorComponent.Deactivate` _niagara)
        (add `NiagaraComponent.OnSystemFinished` _niagara (`|CreateDelegate` :!event `Destroy Actor`))
        (set `local.Bound?` true)))
    (:`else`
      _))
  (bind _object_vfx (`self.Object VFX`)
    (:`then`
      (if (`ActorComponent.IsActive` _object_vfx)
        (`ActorComponent.Deactivate` _object_vfx)
        (add `NiagaraComponent.OnSystemFinished` _object_vfx (`|CreateDelegate` :!event `Destroy Actor`))
        (`KismetSystemLibrary.K2_ClearAndInvalidateTimerHandle` (`self.Trace`))
        (else
          (if (not (`local.Bound?`)) :!label _label
            (`self.K2_DestroyActor`)))))
    (:`else`
      (goto _label))))

(fn `Explode`
  (if (>= (`self.Explosions`) 1)
    (`|SpawnActorFromClass` "/Game/Base/BaseWeapons/Explosions/BP_Explosion.BP_Explosion_C" (`SceneComponent.K2_GetComponentToWorld` (`self.Object`)) "Undefined" "MultiplyWithRoot" null self (struct) 20.0 0.0 null null)
    (bind _result (`/Engine/EditorBlueprintResources/StandardMacros.DecrementInt` (`self.Explosions`))
      (:`  `
        (if (<= _result 0)
          (`self.Destroy Projectile`)
          (else
            (`KismetSystemLibrary.K2_SetTimerDelegate` (`|CreateDelegate` :!event `Explode`) (`/Game/Base/BaseWeapons/Projectiles/DA_Projectile.Explosion Delay` (`self.Data`)))))))))

(fn `Get Direction`
  (returns (ReturnValue :type "Vector Structure"))
  (return (`KismetMathLibrary.Normal` (`self.GetVelocity`))))

(fn `Get Velocity`
  (returns (ReturnValue :type "Vector Structure"))
  (bind _returnvalue (`PrimitiveComponent.GetPhysicsLinearVelocity` (`self.Sphere`) "None"))
  (return _returnvalue))

(fn `Hit Trigger`
  (params (Hit :type "HitResult Structure") (Head :type Boolean))
  (locals (`Last Updated Velocity` :type "Vector Structure" :default (0.0 0.0 0.0)))
  (bind (_bblockinghit _binitialoverlap _time _distance _location _impactpoint _normal _impactnormal _physmat _hitactor) (`GameplayStatics.BreakHitResult` Hit))
  (bind _object (`self.Object`))
  (bind _richochets (`self.Richochets`))
  (bind _object_2 (`self.Object`))
  (bind (_bblockinghit_2 _binitialoverlap_2 _time_2 _distance_2 _location_2 _impactpoint_2 _normal_2 _impactnormal_2) (`GameplayStatics.BreakHitResult` (`local.Hit`)))
  (bind (_bblockinghit_3 _binitialoverlap_3 _time_3 _distance_3 _location_3 _impactpoint_3 _normal_3 _impactnormal_3 _physmat_2 _hitactor_2 _hitcomponent) (`GameplayStatics.BreakHitResult` (`local.Hit`)))
  (bind _returnvalue (`self.Get Velocity`))
  (set `local.Last Updated Velocity` _returnvalue)
  (message `/Game/Base/BaseDamage/Health/BPI_Health.Apply Damage` _hitactor (make `/Game/Base/BaseDamage/Struct_DamageHitResult` (make `/Game/Base/BaseDamage/Struct_Damage` 1.5) Hit (`self.Damage Info Hit Tags`) (`self.Causer`)))
  (if (<= _richochets 0)
    (set `self.IsActive?` false)
    (`self.Stop Rotation`)
    (`ActorComponent.Deactivate` (`self.Niagara`))
    (`KismetSystemLibrary.K2_ClearAndInvalidateTimerHandle` (`self.Physics`))
    (`PrimitiveComponent.SetSimulatePhysics` (`self.Sphere`) false)
    (`self.K2_SetActorLocation` _impactpoint)
    (`|ExecutionSequence`
      (:`then_0`
        (`self.Explode`))
      (:`then_1`
        (if (and (`BlueprintSetLibrary.Set_Contains` (`/Game/Base/BaseWeapons/Projectiles/DA_Projectile.Stick To Surfaces` (`self.Data`)) (`PhysicalMaterial.SurfaceType` _physmat_2)) Head)
          (`SceneComponent.K2_AttachToComponent` (`self.Object`) _hitcomponent "None" "KeepWorld" "KeepWorld" "KeepWorld" true)
          (else
            (`PrimitiveComponent.SetUseCCD` _object true "None")
            (`PrimitiveComponent.SetSimulatePhysics` _object_2 true)
            (`PrimitiveComponent.SetCollisionEnabled` _object_2 "QueryAndPhysics")
            (`PrimitiveComponent.SetPhysicsLinearVelocity` _object (* (`KismetMathLibrary.Normal` _impactnormal_2) (`KismetMathLibrary.VSize` (`local.Last Updated Velocity`)) 0.05) true "None")
            (`PrimitiveComponent.SetPhysicsAngularVelocityInDegrees` _object (`KismetMathLibrary.MakeVector` (.roll (`KismetMathLibrary.MakeRotFromX` (* _impactnormal_2 -2.0))) (.pitch (`KismetMathLibrary.MakeRotFromX` (* _impactnormal_2 -2.0))) (.yaw (`KismetMathLibrary.MakeRotFromX` (* _impactnormal_2 -2.0)))) true "None")))))
    (else
      (`/Engine/EditorBlueprintResources/StandardMacros.DecrementInt` _richochets
        (:`  `
          (`self.Set Projectile Velocity` (`KismetMathLibrary.Conv_RotatorToVector` (`KismetMathLibrary.Conv_VectorToRotator` (`KismetMathLibrary.Normal` _impactnormal))) (* (`KismetMathLibrary.VSize` (`local.Last Updated Velocity`)) (`/Game/Base/BaseWeapons/Projectiles/DA_Projectile.Restitution` (`self.Data`))))
          (`KismetSystemLibrary.K2_SetTimerDelegate` (`|CreateDelegate` :!event `Start Trace`) 0.01))))))

(fn `Initial Trace`
  (returns (`Hit?` :type Boolean))
  (bind _returnvalue (`self.K2_GetActorLocation`))
  (bind (_outhit _returnvalue_2) (`KismetSystemLibrary.SphereTraceSingle` _returnvalue (+ _returnvalue (* (`KismetMathLibrary.Conv_RotatorToVector` (`self.K2_GetActorRotation`)) 300.0)) (`/Game/Base/BaseWeapons/Projectiles/DA_Projectile.Head Radius` (`self.Data`)) "TraceTypeQuery1" false (`self.Actors to Ignore`)))
  (if _returnvalue_2
    (`self.K2_SetActorLocation` (`.ImpactPoint` (`GameplayStatics.BreakHitResult` _outhit)))
    (`self.Hit` _outhit true)
    (return true)
    (else
      (return false))))

(fn `Rotate`
  (bind _objectroot (`self.ObjectRoot`))
  (`SceneComponent.K2_SetRelativeRotation` _objectroot (`KismetMathLibrary.ComposeRotators` (`SceneComponent.RelativeRotation` _objectroot) (`KismetMathLibrary.MakeRotator` (.x (`/Game/Base/BaseWeapons/Projectiles/DA_Projectile.Rotation` (`self.Data`))) (.y (`/Game/Base/BaseWeapons/Projectiles/DA_Projectile.Rotation` (`self.Data`))) (.z (`/Game/Base/BaseWeapons/Projectiles/DA_Projectile.Rotation` (`self.Data`))))) false false))

(fn `Set Projectile Velocity`
  (params (Direction :type "Vector Structure") (Speed :type "Float (double-precision)"))
  (`PrimitiveComponent.SetPhysicsLinearVelocity` (`self.Sphere`) (* Direction Speed) true "None"))

(fn `Start Rotation`
  (bind _returnvalue (`KismetSystemLibrary.K2_SetTimerDelegate` (`|CreateDelegate` :!event `Rotate`) 0.01 true true))
  (set `self.Rotation` _returnvalue))

(fn `Start Trace`
  (set `self.Last Location` (`SceneComponent.GetSocketLocation` (`self.Object`) (`self.Head Start Name`)))
  (bind _returnvalue (`KismetSystemLibrary.K2_SetTimerDelegate` (`|CreateDelegate` :!event `Trace for Hit`) (`self.Trace Time`) true true))
  (set `self.Trace` _returnvalue))

(fn `Stop Rotation`
  (`KismetSystemLibrary.K2_ClearAndInvalidateTimerHandle` (`self.Rotation`)))

(fn `Trace Body`
  (bind (_outhit _returnvalue) (`KismetSystemLibrary.SphereTraceSingle` (`SceneComponent.GetSocketLocation` (`self.Object`) (`self.Body Start Name`)) (`SceneComponent.GetSocketLocation` (`self.Object`) (`self.Body End Name`)) (`/Game/Base/BaseWeapons/Projectiles/DA_Projectile.Head Radius` (`self.Data`)) "TraceTypeQuery1" false (`self.Actors to Ignore`)))
  (if _returnvalue
    (`self.Hit` _outhit)))

(fn `Trace Head`
  (returns (Success :type Boolean))
  (bind (_outhit _returnvalue) (`KismetSystemLibrary.SphereTraceSingle` (`self.Last Location`) (`SceneComponent.GetSocketLocation` (`self.Object`) (`self.Head End Name`)) (`/Game/Base/BaseWeapons/Projectiles/DA_Projectile.Head Radius` (`self.Data`)) "TraceTypeQuery1" false (`self.Actors to Ignore`)))
  (if _returnvalue
    (`self.Hit` _outhit true)
    (return true)
    (else
      (set `self.Last Location` (`.TraceEnd` (`GameplayStatics.BreakHitResult` _outhit)))
      (return false))))

(fn `UserConstructionScript`
  (bind _data (`self.Data`))
  (bind _object (`self.Object`))
  (bind _data_2 (`self.Data`))
  (`NiagaraComponent.SetAsset` (`self.Niagara`) (`/Game/Base/BaseWeapons/Projectiles/DA_Projectile.Trail` _data) true)
  (set `self.Explosions` (`/Game/Base/BaseWeapons/Projectiles/DA_Projectile.Explosions` _data))
  (set `self.Richochets` (`/Game/Base/BaseWeapons/Projectiles/DA_Projectile.Richochets` (`self.Data`)))
  (`StaticMeshComponent.SetStaticMesh` (`self.Object`) (`/Game/Base/BaseWeapons/Projectiles/DA_Projectile.Object` _data_2))
  (`NiagaraComponent.SetAsset` (`self.Object VFX`) (`/Game/Base/BaseWeapons/Projectiles/DA_Projectile.Object VFX` _data_2) true)
  (`SceneComponent.K2_SetRelativeLocation` _object (* (.location (`SceneComponent.GetSocketTransform` _object "Center" "RTS_Component")) -1.0) false false)
  (`SceneComponent.K2_AttachToComponent` (`self.Object VFX`) (`self.Object`) "Center" "SnapToTarget" "SnapToTarget" "SnapToTarget" true)
  (`PrimitiveComponent.SetLinearDamping` (`self.Sphere`) (`/Game/Base/BaseWeapons/Projectiles/DA_Projectile.Friction` (`self.Data`))))