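; BP_Sniper is an attacking character that fires a fast projectile toward its target.
; Attack pauses movement and plays the floating attack montage while activating a Niagara effect as a wind-up.
; The montage's notify spawns a BP_BasicProjectile from the ProjectileSpawn point along the target direction, then switches the effect off.
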(event `self.Attack`
  (`self.Pause Movement` 2.0)
  (`|PlayMontage` (`self.SkeletalMesh`) "/Game/Imports/Sniper2/SkeletalMeshes/Floating_Attack_Montage.Floating_Attack_Montage"
    (:`then`
      (`ActorComponent.Activate` (`self.Niagara`) true))
    (:`OnNotifyBegin`
      (`|SpawnActorFromClass` "/Game/Project/BP_BasicProjectile.BP_BasicProjectile_C" (`KismetMathLibrary.MakeTransform` (`SceneComponent.K2_GetComponentLocation` (`self.Projectile Spawn`)) (`KismetMathLibrary.Conv_VectorToRotator` (`self.Get Target Direction`))) "AlwaysSpawn" "MultiplyWithRoot" null 5000.0 5 null)
      (`ActorComponent.Deactivate` (`self.Niagara`)))))

(fn `UserConstructionScript`
  (`parent.UserConstructionScript`))