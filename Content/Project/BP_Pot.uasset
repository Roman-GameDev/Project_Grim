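; BP_Pot is a breakable pot that can drop collectables.
; When its Health resource empties, it runs SpawnCollectable and then destroys itself.
; SpawnCollectable has an even chance to spawn a random number of BP_Collectable actors at the pot's location, always spawning regardless of collision, each given one of two types at random.
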(event `self.Health.On Resource Empty`
  (`self.Spawn Collectable`)
  (`self.K2_DestroyActor`))

(event `Spawn Collectable`
  (if (< (`KismetMathLibrary.RandomFloat`) 0.5)
    (for _ (range (+ (`KismetMathLibrary.RandomIntegerInRange` 0 5) 1))
      (`|SpawnActorFromClass` "/Game/Project/BP_Collectable.BP_Collectable_C" (`KismetMathLibrary.MakeTransform` (`self.K2_GetActorLocation`)) "AlwaysSpawn" "MultiplyWithRoot" null (`KismetArrayLibrary.Array_Random` (`|MakeArray` "NewEnumerator0" "NewEnumerator1" :!type "/Game/Project/Enum_CollectableType Enum")) null))))

(fn `UserConstructionScript`
  (`parent.UserConstructionScript`))