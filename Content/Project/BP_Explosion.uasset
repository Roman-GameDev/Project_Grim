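; BP_Explosion is a one-shot explosion actor that deals damage and physical knockback around its location when spawned.
; On BeginPlay it plays an epicenter-oriented camera shake and spawns a heavy-impact Niagara effect, both scaled by Radius.
; A radius trace ignoring itself and its Causer finds hit actors, applying health damage and a damage-scaled impulse to each.
; The actor then destroys itself immediately.
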(event `self.ReceiveBeginPlay`
  (bind _damage (`self.Damage`))
  (`GameplayStatics.PlayWorldCameraShake` "/Game/Project/LCS_Explosion.LCS_Explosion_C" (`self.K2_GetActorLocation`) 0.0 (* (`self.Radius`) 2.0) 0.5 true)
  (bind _returnvalue (`NiagaraFunctionLibrary.SpawnSystemAtLocation` "/Game/Project/NS_HeavyImpact.NS_HeavyImpact" (.location (`self.GetTransform`)) (.rotation (`self.GetTransform`))))
  (`NiagaraComponent.SetVariableFloat` _returnvalue "Scale" (/ (`self.Radius`) 50.0))
  (bind _hits_result (`/Game/Project/BFL_General.Explosion Trace` (`self.K2_GetActorLocation`) (`self.Radius`) "TraceTypeQuery1" "None" (`|MakeArray` self (`self.Causer`) :!type "Actor Object Reference")))
  (for _array_element _hits_result
    (message `/Game/Project/BPI_Health.Apply Health Damage` (`.HitActor` (`GameplayStatics.BreakHitResult` _array_element)) _damage)
    (`/Game/Project/BFL_General.Apply Impulse to Hit` _array_element (`KismetMathLibrary.Conv_IntToDouble` (* _damage 100))))
  (`self.K2_DestroyActor`))

(fn `UserConstructionScript`)