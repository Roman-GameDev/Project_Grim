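; BP_Basic is an attacker Blueprint that fires short, randomized bursts of BP_BasicProjectile toward its target.
; Attack resets the burst counter and starts a short timer, apparently leading to Burst, which spawns a projectile at the Spell component within a random cone around the target direction.
; Burst re-arms a timer while the counter is below a freshly rolled random limit, giving one to three shots weighted toward fewer.
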(event `self.ReceiveBeginPlay`
  (`parent.ReceiveBeginPlay`))

(event `self.Attack`
  (set `self.Burst Count` 0)
  (`KismetSystemLibrary.K2_SetTimerDelegate` (`|CreateDelegate` :!event `Burst`) 0.1))

(event `Burst`
  (`|SpawnActorFromClass` "/Game/Project/BP_BasicProjectile.BP_BasicProjectile_C" (`KismetMathLibrary.MakeTransform` (`SceneComponent.K2_GetComponentLocation` (`self.Spell`)) (`KismetMathLibrary.Conv_VectorToRotator` (`KismetMathLibrary.RandomUnitVectorInConeInDegrees` (`self.Get Target Direction`) 15.0))) "AlwaysSpawn" "MultiplyWithRoot" null 1000.0 1 null)
  (if (< (`self.Burst Count`) (`KismetMathLibrary.RandomIntegerInRange` 0 2))
    (`KismetSystemLibrary.K2_SetTimerDelegate` (`|CreateDelegate` :!event `Burst`) 0.1)
    (`/Engine/EditorBlueprintResources/StandardMacros.IncrementInt` (`self.Burst Count`))))

(fn `UserConstructionScript`
  (`parent.UserConstructionScript`))