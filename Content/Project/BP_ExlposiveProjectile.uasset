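; Projectile that flies along its forward vector at a set speed and explodes on impact, with Cull as a timeout path.
; A looping timer drives short sphere traces along the velocity, ignoring itself and its Causer, instead of relying on collision events.
; A hit or Cull enters a DoOnce that spawns BP_Explosion from the last trace result, passing radius and damage, then stops tracing and destroys the projectile.
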(event `self.ReceiveBeginPlay`
  (set `MovementComponent.Velocity` (* (`self.GetActorForwardVector`) (`self.Projectile Speed`)) (`self.ProjectileMovement`))
  (bind _returnvalue (`KismetSystemLibrary.K2_SetTimerDelegate` (`|CreateDelegate` :!event `Trace`) 0.05 true))
  (set `self.Trace Timer Handle` _returnvalue)
  (`KismetSystemLibrary.K2_SetTimerDelegate` (`|CreateDelegate` :!event `Cull`) 5.0))

(event `Cull`
  (`/Engine/EditorBlueprintResources/StandardMacros.DoOnce` false :!label _label
    (:`Completed`
      (bind (_bblockinghit _binitialoverlap _time _distance _location _impactpoint _normal _impactnormal _physmat _hitactor _hitcomponent _hitbonename _bonename _hititem _elementindex _faceindex _tracestart) (`GameplayStatics.BreakHitResult` (stale `Trace` _outhit)))
      (`|SpawnActorFromClass` "/Game/Project/BP_Explosion.BP_Explosion_C" (`KismetMathLibrary.MakeTransform` _tracestart (`KismetMathLibrary.Conv_VectorToRotator` _impactnormal)) "Undefined" "MultiplyWithRoot" null (`self.Radius`) 10 self null)
      (`KismetSystemLibrary.K2_ClearAndInvalidateTimerHandle` (`self.Trace Timer Handle`))
      (`self.K2_DestroyActor`))))

(event `Trace`
  (bind _returnvalue (`SceneComponent.K2_GetComponentLocation` (`self.Sphere`)))
  (bind _returnvalue_2 (`KismetMathLibrary.Normal` (`self.GetVelocity`)))
  (bind (_outhit _returnvalue_3) (`KismetSystemLibrary.SphereTraceSingle` (+ _returnvalue (* _returnvalue_2 -25.0)) (+ _returnvalue (* _returnvalue_2 25.0)) 50.0 "TraceTypeQuery1" false (`|MakeArray` (`self.Causer`) self :!type "Actor Object Reference")))
  (if _returnvalue_3
    (goto _label)))

(fn `UserConstructionScript`)