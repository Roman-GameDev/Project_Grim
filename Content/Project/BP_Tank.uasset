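; BP_Tank is a slow-clap bruiser character that turns into a suicide bomber at low health.
; Its attack pauses movement and plays a montage whose notify spawns BP_Explosion at the Clap component, with left and right effects active during the windup.
; Below 20% health it enrages, retuning speed and range values.
; Enraged attacks and health depletion share a DoOnce-guarded explode montage that spawns a larger explosion and destroys the actor.
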(event `self.ReceiveBeginPlay`
  (`parent.ReceiveBeginPlay`))

(event `self.Attack`
  (`self.Pause Movement` 2.0)
  (if (`self.Is Enraged?`)
    (`/Engine/EditorBlueprintResources/StandardMacros.DoOnce` false :!label _label
      (:`Completed`
        (`|PlayMontage` (`self.SkeletalMesh`) "/Game/Imports/Tank/SkeletalMeshes/Floating_Explode.Floating_Explode"
          (:`then`
            (`ActorComponent.Activate` (`self.E`) true))
          (:`OnNotifyBegin`
            (`|SpawnActorFromClass` "/Game/Project/BP_Explosion.BP_Explosion_C" (`KismetMathLibrary.MakeTransform` (`self.K2_GetActorLocation`)) "Undefined" "MultiplyWithRoot" null 600.0 5 self null)
            (`self.K2_DestroyActor`)))))
    (else
      (`|PlayMontage` (`self.SkeletalMesh`) "/Game/Imports/Tank/SkeletalMeshes/Floating_attack_Montage.Floating_attack_Montage"
        (:`then`
          (`ActorComponent.Activate` (`self.L`) true)
          (`ActorComponent.Activate` (`self.R`) true))
        (:`OnNotifyBegin`
          (`|SpawnActorFromClass` "/Game/Project/BP_Explosion.BP_Explosion_C" (`KismetMathLibrary.MakeTransform` (`SceneComponent.K2_GetComponentLocation` (`self.Clap`))) "Undefined" "MultiplyWithRoot" null 300.0 5 self null)
          (`ActorComponent.Deactivate` (`self.L`))
          (`ActorComponent.Deactivate` (`self.R`)))))))

(event `self.Health.On Resource Lost`
  (params (Current :type Integer) (Ratio :type "Float (double-precision)"))
  (if (< Ratio 0.2)
    (set `self.Speed` 1000.0)
    (set `self.Attack Acceptance` 300.0)
    (set `self.Too Close Radius` 0.0)
    (set `self.Too Close Tolerance` 0.0)
    (set `self.Is Enraged?` true)
    (set `self.Too Far Radius` 200.0)
    (`self.Attack Delay Reset`)))

(event `self.Health.On Resource Empty`
  (goto _label))

(fn `UserConstructionScript`
  (`parent.UserConstructionScript`))