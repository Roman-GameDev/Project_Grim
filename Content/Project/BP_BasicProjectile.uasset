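; BP_BasicProjectile is a projectile actor that damages the player character on contact.
; On BeginPlay it sets its ProjectileMovement velocity along its forward vector, scaled by ProjectileSpeed.
; When Sphere1 overlaps player 0's character, it sends ApplyHealthDamageMessage with Damage, gated by a DoOnce so it hits only once.
; The projectile ignores other actors in that overlap and does not destroy itself in this graph.
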(event `self.ReceiveBeginPlay`
  (set `MovementComponent.Velocity` (* (`self.GetActorForwardVector`) (`self.Projectile Speed`)) (`self.ProjectileMovement`)))

(event `self.Sphere1.OnComponentBeginOverlap`
  (params (OverlappedComponent :type "PrimitiveComponent Object Reference") (OtherActor :type "Actor Object Reference") (OtherComp :type "PrimitiveComponent Object Reference") (OtherBodyIndex :type Integer) (bFromSweep :type Boolean) (SweepResult :type "HitResult Structure (by ref)"))
  (bind _returnvalue (`GameplayStatics.GetPlayerCharacter` 0))
  (if (== OtherActor _returnvalue)
    (`/Engine/EditorBlueprintResources/StandardMacros.DoOnce` false
      (:`Completed`
        (message `/Game/Project/BPI_Health.Apply Health Damage` _returnvalue (`self.Damage`))))))

(fn `UserConstructionScript`)