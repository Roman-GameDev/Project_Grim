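; BP_EnemySpawner is an actor that spawns BP_Enemy instances at random positions inside its Box volume.
; BeginPlay starts a looping timer at the SpawnTimer interval to drive spawning.
; Spawn takes random X and Y from the box and Z from the actor, adjusting for collisions but always spawning.
; A running count stops spawns once it exceeds MaxSpawns, allowing one extra, and never decrements.
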(event `self.ReceiveBeginPlay`
  (`KismetSystemLibrary.K2_SetTimerDelegate` (`|CreateDelegate` :!event `Spawn`) (`self.Spawn Timer`) true))

(event `Spawn`
  (bind _box (`self.Box`))
  (if (not (> (`self.Spawns`) (`self.Max Spawns`)))
    (`|SpawnActorFromClass` "/Game/Project/BP_Enemy.BP_Enemy_C" (`KismetMathLibrary.MakeTransform` (`KismetMathLibrary.MakeVector` (.x (`KismetMathLibrary.RandomPointInBoundingBox` (`SceneComponent.K2_GetComponentLocation` _box) (`BoxComponent.GetScaledBoxExtent` _box))) (.y (`KismetMathLibrary.RandomPointInBoundingBox` (`SceneComponent.K2_GetComponentLocation` _box) (`BoxComponent.GetScaledBoxExtent` _box))) (.z (`self.K2_GetActorLocation`)))) "AdjustIfPossibleButAlwaysSpawn" "MultiplyWithRoot" null null)
    (`/Engine/EditorBlueprintResources/StandardMacros.IncrementInt` (`self.Spawns`))))

(fn `UserConstructionScript`)