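; BP_MovingTarget is an actor that jumps between positions, apparently as a moving target for the wand feature.
; BeginPlay starts a looping one-second timer, whose delegate presumably drives the custom event.
; That event uses a FlipFlop to alternately add one of two offset vectors to the current location, moving the actor instantly without sweep.
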(event `self.ReceiveBeginPlay`
  (`KismetSystemLibrary.K2_SetTimerDelegate` (`|CreateDelegate` :!event `CustomEvent`) 1.0 true))

(event `CustomEvent`
  (`/Engine/EditorBlueprintResources/StandardMacros.FlipFlop`
    (:`A`
      (`self.K2_SetActorLocation` (+ (`self.New Location 1`) (`self.K2_GetActorLocation`))))
    (:`B`
      (`self.K2_SetActorLocation` (+ (`self.New Location`) (`self.K2_GetActorLocation`))))))

(fn `UserConstructionScript`)