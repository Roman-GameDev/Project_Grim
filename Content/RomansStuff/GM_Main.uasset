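; GM_Main runs timed enemy spawning when the GM controller's StartSpawningEnemies flag is set.
; A looping one-second timer spawns more enemies as minutes pass, within a total cap, and adds new types' weights at their spawn times.
; Types are picked by weight, alive counts and per-type caps; EnemyKilled decrements the counts.
; Spawn points come from a ConvertTrace cast horizontally opposite the camera's view at random distance.
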(event `self.ReceiveBeginPlay`
  (bind _returnvalue (`GameplayStatics.GetActorOfClass` "/Game/RomansStuff/BP_GMController.BP_GMController_C"))
  (bind _output_get (set `self.Controller` _returnvalue))
  (if (`/Game/RomansStuff/BP_GMController.Start Spawning Enemies?` _output_get)
    (`KismetSystemLibrary.K2_SetTimerDelegate` (`|CreateDelegate` :!event `Timer`) 1.0 true)
    (for _array_element (`self.Enemies`)
      (`KismetArrayLibrary.Array_Add` (`self.Type Caps`) (`.SpawnCap_5_96077310478B5138D50236ABCB690061` (break `/Game/RomansStuff/Enemy/struct_enemyspawninfo` _array_element))))))

(event `/Game/RomansStuff/BPI_GameMode.Enemy Killed`
  (params (`Index Type` :type Integer))
  (bind _alive_counts (`self.Alive Counts`))
  (`KismetArrayLibrary.Array_Set` _alive_counts `Index Type` (- (`|GetArrayItem` _alive_counts `Index Type`) 1))
  (`/Engine/EditorBlueprintResources/StandardMacros.DecrementInt` (`self.Total Count`)))

(fn `Get Spawn Location`
  (returns (Location :type "Vector Structure"))
  (bind _returnvalue (`GameplayStatics.GetPlayerCameraManager` 0))
  (return (`/Game/Base/BFL_General.Convert Trace` (`PlayerCameraManager.GetCameraLocation` _returnvalue) (* (`KismetMathLibrary.GetForwardVector` (`PlayerCameraManager.GetCameraRotation` _returnvalue)) (-1.0 -1.0 0.0)) (`KismetMathLibrary.RandomFloatInRange` 5000.0 10000.0) 15.0)))

(fn `Spawn Enemy`
  (params (Selected :type Integer))
  (`|SpawnActorFromClass` "/Game/Project/BP_Enemy.BP_Enemy_C" (`KismetMathLibrary.MakeTransform` (`self.Get Spawn Location`)) "AlwaysSpawn" "MultiplyWithRoot" null (`.Data_2_2D8CE36C49AFEDDF7A139FACA502AE00` (break `/Game/RomansStuff/Enemy/struct_enemyspawninfo` (`|GetArrayItem` (`self.Enemies`) Selected))) Selected null))

(fn `Timer`
  (locals (Selected :type Integer :default 0))
  (bind _current_spawn_weights (`self.Current Spawn Weights`))
  (bind _total_count (`self.Total Count`))
  (bind _max_count (`self.Max Count`))
  (bind _enemies (`self.Enemies`))
  (bind _selected (`local.Selected`))
  (bind _alive_counts (`self.Alive Counts`))
  (bind _returnvalue (+ (`KismetArrayLibrary.Array_LastIndex` _current_spawn_weights) 1))
  (`|ExecutionSequence`
    (:`then_0`
      (if (not (>= _total_count _max_count))
        (for _ (range 1 (+ (`KismetMathLibrary.Clamp` (`.Minutes` (`KismetMathLibrary.BreakTimespan` (`KismetMathLibrary.FromSeconds` (`KismetSystemLibrary.GetGameTimeInSeconds`)))) 1 (- _max_count _total_count)) 1))
          (bind _returnvalue_2 (`GrimSpawnLibrary.ChooseWeightedEnemyType` (`self.Current Spawn Weights`) (`self.Alive Counts`) (`self.Type Caps`)))
          (bind _output_get (set `local.Selected` _returnvalue_2))
          (if (>= _output_get 0)
            (`KismetArrayLibrary.Array_Set` _alive_counts _selected (+ (`|GetArrayItem` _alive_counts _selected) 1) true)
            (`/Engine/EditorBlueprintResources/StandardMacros.IncrementInt` (`self.Total Count`)
              (:`  `
                (`self.Spawn Enemy` (`local.Selected`))))))))
    (:`then_1`
      (if (and (> (`KismetSystemLibrary.GetGameTimeInSeconds`) (`.SpawnTime_9_0E4FB51F408EF9E7123FB48EA2B435AF` (break `/Game/RomansStuff/Enemy/struct_enemyspawninfo` (`|GetArrayItem` _enemies _returnvalue)))) (< (`KismetArrayLibrary.Array_Length` _current_spawn_weights) (`KismetArrayLibrary.Array_Length` _enemies)))
        (`KismetArrayLibrary.Array_Set` (`self.Current Spawn Weights`) _returnvalue (`.SpawnWeight_11_414E8A01427B0B3968CE61BA1EA46899` (break `/Game/RomansStuff/Enemy/struct_enemyspawninfo` (`|GetArrayItem` (`self.Enemies`) _returnvalue))) true)))))

(fn `UserConstructionScript`)