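; Test actor that previews a configurable skeletal mesh and animation, apparently for checking head-tracking data.
; The construction script assigns the mesh and animation, and BeginPlay plays the animation looping.
; Unconnected debug draws would compare a sampled HeadPositions entry, indexed by playback time and sample rate, against the live "HT" socket using colored spheres.
; Tick is empty, so that comparison never runs.
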(event `self.ReceiveBeginPlay`
  (`SkeletalMeshComponent.PlayAnimation` (`self.SkeletalMesh`) (`self.animation`) true))

(event `self.ReceiveTick`
  (params (DeltaSeconds :type "Float (single-precision)")))

(fn `UserConstructionScript`
  (bind _skeletalmesh (`self.SkeletalMesh`))
  (`SkeletalMeshComponent.SetSkeletalMeshAsset` _skeletalmesh (`self.Mesh`))
  (set `SkeletalMeshComponent.AnimationData` (make `SingleAnimationPlayData` (`self.animation`)) _skeletalmesh))